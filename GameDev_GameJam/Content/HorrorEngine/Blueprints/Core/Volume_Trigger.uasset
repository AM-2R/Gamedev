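; Volume_Trigger is a box trigger volume that activates linked actors and horror events when something begins overlapping it.
; On overlap it runs an interaction check, then, if not yet opened, waits a configurable delay and calls OpenOn on its ActorsToUse.
; It then runs a horror event check and sets an Opened flag after the delay, so later overlaps skip the activation.
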(event `self.Box.OnComponentBeginOverlap`
  (params (OverlappedComponent :type "PrimitiveComponent Object Reference") (OtherActor :type "Actor Object Reference") (OtherComp :type "PrimitiveComponent Object Reference") (OtherBodyIndex :type Integer) (bFromSweep :type Boolean) (SweepResult :type "HitResult Structure (by ref)"))
  (`/Game/HorrorEngine/Blueprints/Core/HorrorEngineMacros.HM_CheckInteraction`)
  (if (not (`self.Opened`))
    (`KismetSystemLibrary.Delay` (`self.Delay`))
    (`self.Open/On` (`self.Actors To Use`) false)
    (`self.HorrorEventCheck` "NewEnumerator3")
    (set `self.Opened` true)))

(fn `UserConstructionScript`
  (`parent.UserConstructionScript`))